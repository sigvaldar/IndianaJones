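; Pressure plate that, when the player steps on it, triggers its linked door, arrow trap or moving wall, selected by ObjectAtachement.
; Door plates light their indicator, then DoorsOpen counts active BP_indicateur_activation actors sharing the door's ID and plays the opening timeline when the required count matches.
; Arrow plates spawn projectiles; wall plates run a timeline that calls the wall's animation through a delay.
; NombreValidation resets only on a successful door check.
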(event OnComponentBeginOverlap(Box)
  (params (OverlappedComponent :type Primitive%20Component%20Object%20Reference) (OtherActor :type Actor%20Object%20Reference) (OtherComp :type Primitive%20Component%20Object%20Reference) (OtherBodyIndex :type Integer) (bFromSweep :type Boolean) (SweepResult :type Hit%20Result%20Structure%20%28by%20ref%29))
  (Utilities|IsPlayer OtherActor
    (:IsPlayer
      (switch string (Variables|Default|GetObjectAtachement)
        (:porte
          ;[1 0.2077 0.2376] Changement de la couleur de l'indicateur d'activation => passe de inactif à activer.
          (Variables|/Game/triggerThings/BP_indicateur_activation.BP_indicateur_activation_C|SetActivation (Variables|Lighter|GetMyLightOn) true)
          (Default|ChangeColor (Variables|Lighter|GetMyLightOn))
          ;[0.06569 0.07899 1] Code permettant le deplacement d'une porte (animation) apres la validation des conditions requise (lorsque tout les indicateur sont actif).
          (Utilities|FlowControl|DoOnce false
            (:Completed
              (bind _isopen (CallFunction|DoorsOpen))
              (if _isopen
                (bind _animationporte (Timeline|TimelinePorte Play)
                  (:Update
                    (Default|AnimationPorte (Variables|Doors|GetMyTriggerDoors) _animationporte)))))))
        (:arrow
          ;[1 1 1] permet de faire spwaner des fleches
          (Default|SpawnProjectile (Variables|Arrow|GetMyTriggerTrapArrows)))
        (:Wall
          ;[1 1 1] Deplacement du mur.
          (Timeline|TimelineWall Play
            (:Update
              (Utilities|FlowControl|Delay 1.0)
              (Default|AnimationMur (Variables|wall|GetMyTriggerWall)))))))))

(fn ConstructionScript)

(fn PressurePActive
  ;[0.63 0 0] Permet de mettre la valeur de la Variable "Activation" à true
  (bind _outactors (Actor|GetAllActorsOfClass "/Game/triggerThings/BP_indicateur_activation.BP_indicateur_activation_C"))
  (Variables|/Game/triggerThings/BP_indicateur_activation.BP_indicateur_activation_C|SetActivation (Utilities|Array|Get(acopy) _outactors) true))

(fn DoorsOpen
  ;[1 1 1] Creation d'une boucle pour chaque objet selectionnés
  (bind _outactors (Actor|GetAllActorsOfClass "/Game/triggerThings/BP_indicateur_activation.BP_indicateur_activation_C"))
  (for _array_element _outactors
    ;[0 1 0.6955] Permet d'ajouter "1" à la variable "Nombre Validation" selon une double condition.
    (if (and (Variables|/Game/triggerThings/BP_indicateur_activation.BP_indicateur_activation_C|GetActivation _array_element) (== (Variables|/Game/triggerThings/BP_Doors.BP_Doors_C|GetidPorte (Variables|Doors|GetMyTriggerDoors)) (Variables|/Game/triggerThings/BP_indicateur_activation.BP_indicateur_activation_C|GetIdLinkDoors _array_element)))
      (bind _result (Math|Float|IncrementFloat (Variables|Doors|GetNombre%20Validation))
        (:%20%20
          (Development|PrintString (Utilities|String|ToString(Float) _result) true true "(R=0.520000,G=0.000000,B=0.000000,A=1.000000)" 1e+01)))))
  ;[1 0 0] renvois True et met la var "Nombre Validation" à 0 si la condition est remplie (comparesion entre 2 varribles).
  (if (== (Variables|Doors|GetNombre%20Validation) (Math|Conversions|ToFloat(Integer) (Variables|/Game/triggerThings/BP_Doors.BP_Doors_C|GetActivateneed (Variables|Doors|GetMyTriggerDoors))))
    (Variables|Doors|SetNombre%20Validation 0.0)
    (return true)))