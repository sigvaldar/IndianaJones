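; BP_StanLee is a collectible Stan Lee statue artefact that the player picks up with the Interact input.
; Overlapping its sphere prints a French pickup prompt, and a gate lets the input through only while the player is inside.
; On pickup, it stores its starting location and scale, then a timeline lerps it toward the player's current position while shrinking it to zero, and destroys the actor when finished.
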(event OnComponentBeginOverlap(StanLee_Sphere)
  (params (OverlappedComponent :type Primitive%20Component%20Object%20Reference) (OtherActor :type Actor%20Object%20Reference) (OtherComp :type Primitive%20Component%20Object%20Reference) (OtherBodyIndex :type Integer) (bFromSweep :type Boolean) (SweepResult :type Hit%20Result%20Structure%20%28by%20ref%29))
  ;[1 1 1] ramasse
  (Development|PrintString "Appuies sur E pour ramasser." true true "(R=1.000000,G=0.015653,B=0.000000,A=1.000000)" 5.0)
  (Utilities|IsPlayer OtherActor
    (:IsPlayer
      (Utilities|FlowControl|Gate true) ; enters at Open
    )))

(event OnComponentEndOverlap(StanLee_Sphere)
  (params (OverlappedComponent :type Primitive%20Component%20Object%20Reference) (OtherActor :type Actor%20Object%20Reference) (OtherComp :type Primitive%20Component%20Object%20Reference) (OtherBodyIndex :type Integer))
  ;[1 1 1] ramasse
  (Utilities|IsPlayer OtherActor
    (:IsPlayer
      (Utilities|FlowControl|Gate true) ; enters at Close
    )))

(event EventBeginPlay
  ;[1 1 1] ramasse
  (Input|EnableInput (Game|GetPlayerController 0)))

(event Input|ActionEvents|InputActionInteract
  (params (Key :type Key%20Structure :default "None"))
  ;[1 1 1] ramasse
  (:Pressed
    (Utilities|FlowControl|Gate true
      (:Exit
        (Development|PrintString "Ramassé")
        (CallFunction|StoreStartingValues)
        (bind (_direction _collection_porgress _scale_progess) (Timeline|Collection%20TimeLine Play)
          (:Update
            (CallFunction|MovetoPlayer _collection_porgress)
            (CallFunction|ScaleStatue _scale_progess))
          (:Finished
            (Actor|DestroyActor)))))))

(fn ConstructionScript)

(fn MovetoPlayer
  (params (Alpha :type Float%20%28single-precision%29))
  (Transformation|SetActorLocation (Math|Vector|Lerp(Vector) (Variables|Default|GetStart%20Location) (Transformation|GetActorLocation (Game|Player|GetPlayerPawn 0)) Alpha) false false))

(fn StoreStartingValues
  (Variables|Default|SetStart%20Location (Transformation|GetActorLocation))
  (Variables|Default|SetStart%20Scale (Transformation|GetActorScale3D)))

(fn ScaleStatue
  (params (Alpha :type Float%20%28single-precision%29))
  (Transformation|SetActorScale3D (Math|Vector|Lerp(Vector) (Variables|Default|GetStart%20Scale) "0, 0, 0" Alpha)))