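; Interactable button that triggers a linked door, arrow trap or moving wall, chosen by its attachment type.
; Box overlap opens a gate for the player's Interact input, which plays a sound and lerps the button in and out.
; Doors light an indicator, then open via timeline if active indicators sharing the door's ID match its required count.
; Arrow traps spawn projectiles, while walls animate through a delayed timeline update.
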(event OnComponentBeginOverlap(Box)
  (params (OverlappedComponent :type Primitive%20Component%20Object%20Reference) (OtherActor :type Actor%20Object%20Reference) (OtherComp :type Primitive%20Component%20Object%20Reference) (OtherBodyIndex :type Integer) (bFromSweep :type Boolean) (SweepResult :type Hit%20Result%20Structure%20%28by%20ref%29))
  ;[1 0.1146 0.6587] Interaction
  (Development|PrintString "Appuyez sur E pour activer le bouton." true true "(R=0.015756,G=1.000000,B=0.000000,A=1.000000)" 5.0)
  (Utilities|IsPlayer OtherActor
    (:IsPlayer
      (Utilities|FlowControl|Gate true) ; enters at Open
    )))

(event OnComponentEndOverlap(Box)
  (params (OverlappedComponent :type Primitive%20Component%20Object%20Reference) (OtherActor :type Actor%20Object%20Reference) (OtherComp :type Primitive%20Component%20Object%20Reference) (OtherBodyIndex :type Integer))
  ;[1 0.1146 0.6587] Interaction
  (Utilities|IsPlayer OtherActor
    (:IsPlayer
      (Utilities|FlowControl|Gate true) ; enters at Close
    )))

(event EventBeginPlay
  (bind _button (Variables|Default|GetButton))
  (bind _returnvalue (Transformation|GetRelativeTransform _button))
  (Variables|Default|SetOut%20Position (Math|Transform|MakeTransform (.location _returnvalue) (.rotation _returnvalue) (.scale _returnvalue)))
  (Variables|Default|SetIn%20Position (Math|Transform|MakeTransform (- (.location _returnvalue) (Math|Vector|MakeVector (Variables|Default|GetXBouton) (Variables|Default|GetYBouton) (Variables|Default|GetZBouton))) (.rotation _returnvalue) (.scale _returnvalue)))
  (Input|EnableInput (Game|GetPlayerController 0)))

(event Input|ActionEvents|InputActionInteract
  (params (Key :type Key%20Structure :default "None"))
  ;[1 0.1146 0.6587] Interaction
  (:Pressed
    (Utilities|FlowControl|Gate true
      (:Exit
        ;[0 1 0.4187] Animation Bouton
        (|ButtonAnimation
          (:Out
            (switch string (Variables|Default|GetObjectAtachement)
              (:porte
                ;[1 0.2077 0.2376] Changement de la couleur de l'indicateur d'activation => passe de inactif à activer.
                (Variables|/Game/triggerThings/BP_indicateur_activation.BP_indicateur_activation_C|SetActivation (Variables|Lighter|GetMyLightOn) true)
                (Default|ChangeColor (Variables|Lighter|GetMyLightOn))
                ;[0.06569 0.07899 1] Code permettant le deplacement d'une porte (animation) apres la validation des conditions requise (lorsque tout les indicateur sont actif).
                (Utilities|FlowControl|DoOnce false
                  (:Completed
                    (bind _isopen (CallFunction|DoorsOpen))
                    (if _isopen
                      (bind _animationporte (Timeline|Timeline_3 Play)
                        (:Update
                          (Default|AnimationPorte (Variables|Doors|GetMyTriggerDoors) _animationporte)))))))
              (:arrow
                ;[1 1 1] permet de faire spwaner des fleches
                (Default|SpawnProjectile (Variables|Arrow|GetMyTriggerTrapArrows)))
              (:Wall
                ;[1 1 1] Deplacement du mur.
                (Timeline|Timeline_4 Play
                  (:Update
                    (Utilities|FlowControl|Delay 1.0)
                    (Default|AnimationMur (Variables|Wall|GetMyTriggerWall))))))))))))

(fn ConstructionScript)

(fn DoorsOpen
  ;[1 1 1] Creation d'une boucle pour chaque objet selectionnés
  (bind _outactors (Actor|GetAllActorsOfClass "/Game/triggerThings/BP_indicateur_activation.BP_indicateur_activation_C"))
  (for _array_element _outactors
    ;[0 1 0.6955] Permet d'ajouter "1" à la variable "Nombre Validation" selon une double condition.
    (if (and (Variables|/Game/triggerThings/BP_indicateur_activation.BP_indicateur_activation_C|GetActivation _array_element) (== (Variables|/Game/triggerThings/BP_Doors.BP_Doors_C|GetidPorte (Variables|Doors|GetMyTriggerDoors)) (Variables|/Game/triggerThings/BP_indicateur_activation.BP_indicateur_activation_C|GetIdLinkDoors _array_element)))
      (bind _result (Math|Float|IncrementFloat (Variables|Doors|GetNombre%20Validation))
        (:%20%20
          (Development|PrintString (Utilities|String|ToString(Float) _result) true true "(R=0.520000,G=0.000000,B=0.000000,A=1.000000)" 1e+01)))))
  ;[1 0 0] renvois True et met la var "Nombre Validation" à 0 si la condition est remplie (comparesion entre 2 varribles).
  (if (== (Variables|Doors|GetNombre%20Validation) (Math|Conversions|ToFloat(Integer) (Variables|/Game/triggerThings/BP_Doors.BP_Doors_C|GetActivateneed (Variables|Doors|GetMyTriggerDoors))))
    (Variables|Doors|SetNombre%20Validation 0.0)
    (return true)))