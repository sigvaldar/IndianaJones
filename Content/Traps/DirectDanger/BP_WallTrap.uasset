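; BP_WallTrap is a wall trap that applies damage to any actor that begins overlapping its BoxCollision.
; AnimationMur shifts the Mur component in world space along the axis chosen by MovementDirection, using MouvementValue.
; Y and Z subtract the value from the current coordinate, while X subtracts the coordinate from the value.
; Nothing in these graphs calls AnimationMur.
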(event OnComponentBeginOverlap(BoxCollision)
  (params (OverlappedComponent :type Primitive%20Component%20Object%20Reference) (OtherActor :type Actor%20Object%20Reference) (OtherComp :type Primitive%20Component%20Object%20Reference) (OtherBodyIndex :type Integer) (bFromSweep :type Boolean) (SweepResult :type Hit%20Result%20Structure%20%28by%20ref%29))
  (Game|Damage|ApplyDamage OtherActor 1.0 0 0))

(fn ConstructionScript)

(fn AnimationMur
  (bind _mur (Variables|Default|Getmur))
  (bind _mur_2 (Variables|Default|Getmur))
  (bind _mur_3 (Variables|Default|Getmur))
  (bind _returnvalue (Transformation|GetWorldLocation _mur_3))
  (bind _returnvalue_2 (Transformation|GetWorldLocation _mur))
  (bind _returnvalue_3 (Transformation|GetWorldLocation _mur_2))
  ;[1 0.6824 0.06772] Permet de modifier la position d'un mur en fonction d'une varriable donnée.
  (switch string (Variables|Default|GetMovementDirection)
    (:Z
      (Transformation|SetWorldLocation (Variables|Default|Getmur) (Math|Vector|MakeVector (.x _returnvalue) (.y _returnvalue) (- (.z _returnvalue) (Variables|Default|GetMouvementValue))) false false))
    (:Y
      (Transformation|SetWorldLocation (Variables|Default|Getmur) (Math|Vector|MakeVector (.x _returnvalue_2) (- (.y _returnvalue_2) (Variables|Default|GetMouvementValue)) (.z _returnvalue_2)) false false))
    (:X
      (Transformation|SetWorldLocation (Variables|Default|Getmur) (Math|Vector|MakeVector (- (Variables|Default|GetMouvementValue) (.x _returnvalue_3)) (.y _returnvalue_3) (.z _returnvalue_3)) false false))))